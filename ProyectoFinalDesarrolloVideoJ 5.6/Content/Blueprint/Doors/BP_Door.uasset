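; An interactable door that the player swings open or closed with the E key while standing near it.
; A Box overlap with BP_ThirdPersonLasso2 enables input and shows an interaction widget; leaving disables input and removes it.
; E toggles a FlipFlop that plays or reverses the DoorOpen timeline, lerping the Arrow component's yaw between closed and open values.
; Opening plays its sound immediately; closing plays another after a short delay.
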(event OnComponentBeginOverlap(Box)
  (params (OverlappedComponent :type Primitive%20Component%20Object%20Reference) (OtherActor :type Actor%20Object%20Reference) (OtherComp :type Primitive%20Component%20Object%20Reference) (OtherBodyIndex :type Integer) (bFromSweep :type Boolean) (SweepResult :type Hit%20Result%20Structure%20%28by%20ref%29))
  ;[0.7007 1 0.3325] INTERACTION
  ;;[0.7007 1 0.3325] Inside the box?
  ;;[0.7007 1 0.3325] Character inside the box
  (Utilities|Casting|CastToBP_ThirdPersonLasso2 OtherActor)
  (Input|EnableInput (Game|GetPlayerController 0))
  ;;[0.7007 1 0.3325] Show Interface
  (bind _returnvalue (UserInterface|CreateWidget "/Game/Widgets/InteractiveInterface.InteractiveInterface_C"))
  (UserInterface|Viewport|AddtoViewport _returnvalue 0))

(event OnComponentEndOverlap(Box)
  (params (OverlappedComponent :type Primitive%20Component%20Object%20Reference) (OtherActor :type Actor%20Object%20Reference) (OtherComp :type Primitive%20Component%20Object%20Reference) (OtherBodyIndex :type Integer))
  ;[0.7007 1 0.3325] INTERACTION
  ;;[0.7007 1 0.3325] Outside the box?
  ;;[0.7007 1 0.3325] Character outside the box
  (Utilities|Casting|CastToBP_ThirdPersonLasso2 OtherActor)
  ;;[0.7007 1 0.3325] Deactivate Input
  (Input|DisableInput (Game|GetPlayerController 0))
  ;;[0.7007 1 0.3325] Quit interface
  (Widget|RemovefromParent (stale OnComponentBeginOverlap(Box) _returnvalue)))

(event Input|KeyboardEvents|E
  (params (Key :type Key%20Structure :default "None"))
  ;[0.7007 1 0.3325] Whats gonna happen?
  (:Pressed
    (Utilities|FlowControl|FlipFlop
      (:A
        (Audio|Components|Audio|Stop (Variables|Default|GetDoorSound))
        (Audio|Components|Audio|Play (Variables|Default|GetDoorSound) 0.0)
        (bind _animdoor (Timeline|Door%20Open Play)
          (:Update
            (Transformation|SetRelativeRotation (Variables|Default|GetArrow) (Math|Rotator|MakeRotator 0.0 0.0 (Math|Float|Lerp (Variables|Default|GetClose%20Door) (Variables|Default|GetOpen%20Door) _animdoor)) false false))))
      (:B
        (Utilities|FlowControl|Sequence
          (:then_0
            (Timeline|Door%20Open Reverse))
          (:then_1
            (Utilities|FlowControl|Delay 0.2)
            (Audio|Components|Audio|Stop (Variables|Default|GetDoorCloseSound))
            (Audio|Components|Audio|Play (Variables|Default|GetDoorCloseSound) 0.0)))))))

(fn ConstructionScript)