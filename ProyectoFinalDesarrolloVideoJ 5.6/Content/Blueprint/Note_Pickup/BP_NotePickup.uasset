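; BP_NotePickup is a collectible note for level 1 that the player picks up by pressing E while standing in its box.
; The box overlap enables player input on the actor when BP_ThirdPersonLasso2 enters and disables it on exit.
; On pickup it decrements NotesLeft on the level 1 game mode, shows two note-collect widgets, destroys itself and plays a page-turn sound.
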(event OnComponentBeginOverlap(Box)
  (params (OverlappedComponent :type Primitive%20Component%20Object%20Reference) (OtherActor :type Actor%20Object%20Reference) (OtherComp :type Primitive%20Component%20Object%20Reference) (OtherBodyIndex :type Integer) (bFromSweep :type Boolean) (SweepResult :type Hit%20Result%20Structure%20%28by%20ref%29))
  (Utilities|Casting|CastToBP_ThirdPersonLasso2 OtherActor)
  (Input|EnableInput (Game|GetPlayerController 0)))

(event OnComponentEndOverlap(Box)
  (params (OverlappedComponent :type Primitive%20Component%20Object%20Reference) (OtherActor :type Actor%20Object%20Reference) (OtherComp :type Primitive%20Component%20Object%20Reference) (OtherBodyIndex :type Integer))
  (Utilities|Casting|CastToBP_ThirdPersonLasso2 OtherActor)
  (Input|DisableInput (Game|GetPlayerController 0)))

(event Input|KeyboardEvents|E
  (params (Key :type Key%20Structure :default "None"))
  (:Pressed
    (bind _asbp_third_person_game_mode_lvl_1 (Utilities|Casting|CastToBP_ThirdPersonGameModeLvl1 (Game|GetGameMode)))
    (bind _result (Math|Integer|DecrementInt (Variables|/Game/ThirdPerson/Blueprints/BP_ThirdPersonGameModeLvl1.BP_ThirdPersonGameModeLvl1_C|GetNotesLeft _asbp_third_person_game_mode_lvl_1))
      (:%20%20
        (Variables|/Game/ThirdPerson/Blueprints/BP_ThirdPersonGameModeLvl1.BP_ThirdPersonGameModeLvl1_C|SetNotesLeft _asbp_third_person_game_mode_lvl_1 _result)
        (bind _returnvalue (UserInterface|CreateWidget "/Game/Widgets/NoteCollect_Widget.NoteCollect_Widget_C"))
        (UserInterface|Viewport|AddtoViewport _returnvalue 0)
        (bind _returnvalue_2 (UserInterface|CreateWidget "/Game/Widgets/NoteCollectLvl1_1_Widget.NoteCollectLvl1_1_Widget_C"))
        (UserInterface|Viewport|AddtoViewport _returnvalue_2 0)
        (Actor|DestroyActor)
        (Audio|PlaySound2D "/Game/Sounds/SoundEffects/Notes/turned-page_Cue.turned-page_Cue" 1.0 1.0 0.0 0 0)))))

(fn ConstructionScript)