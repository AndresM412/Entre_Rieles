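; BP_Dialogue is a dialogue Blueprint that shows lines from data tables in a WB_Dialogue widget.
; Each NewFunction call creates the widget, updates the existing one, or removes it once EndDialogue is set.
; Creation passes Name as speaker and the row's text, then stores that row's next row, table and end flag.
; The update branch looks up by Name and calls UpdateDialogue without passing text or advancing state.
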(event EventBeginPlay)

(event EventTick
  (params (DeltaSeconds :type Float%20%28single-precision%29)))

(event EventNewFunction
  (params (PlayerREF :type BP%20Third%20Person%20Lasso%202%20Object%20Reference))
  (if (Variables|Default|GetEnd_Dialogue)
    (Widget|RemovefromParent (Variables|Default|GetDialogue_Widget))
    (Variables|Default|SetEnd_Dialogue false)
    (Variables|Default|SetDialogue_Widget 0)
    (else
      (Utilities|IsValid (Variables|Default|GetDialogue_Widget)
        (:Is%20Valid
          (bind _returnvalue (Utilities|GetDataTableRow (Variables|Default|GetData%20Table) (Variables|Default|GetName))
            (:then
              (Default|UpdateDialogue (Variables|Default|GetDialogue_Widget)))))
        (:Is%20Not%20Valid
          (bind _returnvalue_2 (Utilities|GetDataTableRow (Variables|Default|GetData%20Table) (Variables|Default|GetRow%20Name))
            (:then
              (bind _returnvalue_3 (UserInterface|CreateWidget "/Game/Dialogue/WB_Dialogue.WB_Dialogue_C" 0 (Utilities|Text|ToText(Name) (Variables|Default|GetName)) (.Dialogue (Utilities|Struct|BreakDialogue_Structure _returnvalue_2))))
              (bind _output_get (Variables|Default|SetDialogue_Widget _returnvalue_3))
              (UserInterface|Viewport|AddtoViewport _output_get 0)
              (Variables|Default|SetRow%20Name (.Row (Utilities|Struct|BreakDialogue_Structure _returnvalue_2)))
              (Variables|Default|SetData%20Table (.Data_Table (Utilities|Struct|BreakDialogue_Structure _returnvalue_2)))
              (Variables|Default|SetEnd_Dialogue (.End_Dialogue (Utilities|Struct|BreakDialogue_Structure _returnvalue_2))))))))))